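; Test AI Blueprint that reacts to pawn sensing and issues AI move orders.
; Seeing a pawn prints a message and sets a Range flag for five seconds.
; A custom update event moves the controlled pawn toward the player controller while Range is set, otherwise issues a targetless move guarded by InMovement.
; A second custom event moves self toward a given BP_Knight; leftover casts and a random-vector node are unused.
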(event `CustomEvent_1`
  (params (Pawn :type "Pawn Object Reference"))
  (bind _asbp_knight (cast `/Game/RPG/Characters/Character/BP_Knight` Pawn))
  (`|AIMoveTo` self (0.0 0.0 0.0) _asbp_knight))

(event `CustomEvent`
  (params (DeltaSeconds :type "Float (double-precision)"))
  (if (`self.Range`)
    (`|AIMoveTo` (`Controller.K2_GetPawn`) (0.0 0.0 0.0) (`GameplayStatics.GetPlayerController` 0) 10.0)
    (elif (not (`self.InMovement`))
      (`|AIMoveTo` (`Controller.K2_GetPawn`) (0.0 0.0 0.0) null 100.0
        (:`then`
          (set `self.InMovement` true))
        (:`OnSuccess`
          (set `self.InMovement` false :!label _label))
        (:`OnFail`
          (goto _label))))))

(event `self.PawnSensing.OnSeePawn`
  (params (Pawn :type "Pawn Object Reference"))
  (`KismetSystemLibrary.PrintText` "I see you!")
  (set `self.Range` true)
  (`KismetSystemLibrary.Delay` 5.0)
  (set `self.Range` false))

(fn `UserConstructionScript`)