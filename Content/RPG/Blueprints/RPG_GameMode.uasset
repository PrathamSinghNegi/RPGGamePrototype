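; RPG game mode that runs a minutes-and-seconds countdown and ends play when time runs out.
; BeginPlay adds a TimeWidget to the viewport.
; Tick uses a one-second Delay as a throttle to decrement Seconds, rolling over into Minutes.
; When both reach zero, it shows the Game_Over widget and pauses the game.
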(event `self.ReceiveBeginPlay`
  (bind _returnvalue (`|CreateWidget` "/Game/RPG/Blueprints/TimeWidget.TimeWidget_C"))
  (`UserWidget.AddToViewport` _returnvalue 0))

(event `self.ReceiveTick`
  (params (DeltaSeconds :type "Float (single-precision)"))
  ;[1 1 1] Count_Down
  (`KismetSystemLibrary.Delay` 1.0)
  (if (== (`self.Seconds`) 0)
    (if (== (`self.Minutes`) 0)
      (bind _returnvalue (`|CreateWidget` "/Game/RPG/Blueprints/Game_Over1/Game_Over.Game_Over_C"))
      (`UserWidget.AddToViewport` _returnvalue 0)
      (`WidgetLayoutLibrary.GetMousePositionOnViewport`)
      (`GameplayStatics.SetGamePaused` true)
      (else
        (set `self.Seconds` 59)
        (set `self.Minutes` (- (`self.Minutes`) 1))))
    (else
      (set `self.Seconds` (- (`self.Seconds`) 1)))))

(fn `UserConstructionScript`)