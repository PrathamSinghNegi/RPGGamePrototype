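; Zombie enemy character that switches between walk and run speed by combat state and is destroyed when its health runs out.
; Mesh hits remove one health and pawn sightings raise speed, both setting a combat flag that clears after a delay.
; Tick applies the speed, handles death and regenerates health through a Delay while below maximum.
; The body-colour dynamic material setup is disconnected and never runs.
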(event `self.ReceiveBeginPlay`
  ;[1 1 1] Start: Speed
  (set `CharacterMovementComponent.MaxWalkSpeed` (`KismetMathLibrary.Conv_IntToDouble` (`self.Walk_Speed`)) (`self.CharacterMovement`)))

(event `self.Mesh.OnComponentHit`
  (params (HitComponent :type "PrimitiveComponent Object Reference") (OtherActor :type "Actor Object Reference") (OtherComp :type "PrimitiveComponent Object Reference") (NormalImpulse :type "Vector Structure") (Hit :type "HitResult Structure (by ref)"))
  (bind _returnvalue (- (`self.Health`) 1))
  ;[1 1 1] Damage: isDead/inCombat
  (if (not (`self.isDead`))
    (`KismetSystemLibrary.PrintText` "You've taken away 1 heath!" true false (struct :`R` 0.913965 :`G` 0.318458 :`B` 1.0 :`A` 1.0))
    (set `self.Health` _returnvalue)
    (if (not (<= _returnvalue 0))
      (set `self.isCombat` true)
      (`KismetSystemLibrary.Delay` 15.0)
      (set `self.isCombat` false))))

(event `self.PawnSensing.OnSeePawn`
  (params (Pawn :type "Pawn Object Reference"))
  ;[1 1 1] To See Player: inCombat/runSpeed
  (set `CharacterMovementComponent.MaxWalkSpeed` (`KismetMathLibrary.Conv_IntToDouble` (`self.Run_Speed`)) (`self.CharacterMovement`))
  (set `self.isCombat` true)
  (`KismetSystemLibrary.Delay` 5.0)
  (set `self.isCombat` false))

(event `self.ReceiveTick`
  (params (DeltaSeconds :type "Float (single-precision)"))
  ;[1 1 1] Speed Mode Character
  (if (`self.isCombat`)
    (set `CharacterMovementComponent.MaxWalkSpeed` (`KismetMathLibrary.Conv_IntToDouble` (`self.Run_Speed`)) (`self.CharacterMovement`))
    (else
      (set `CharacterMovementComponent.MaxWalkSpeed` (`KismetMathLibrary.Conv_IntToDouble` (`self.Walk_Speed`)) (`self.CharacterMovement`))))
  ;[1 1 1] Dead Character
  (if (<= (`self.Health`) 0)
    (set `self.isCombat` false)
    (set `self.isDead` true)
    (`self.K2_DestroyActor`)
    (`KismetSystemLibrary.PrintText` "You are kill mob!" true false (struct :`R` 1.0 :`G` 0.741034 :`B` 0.04517 :`A` 1.0))
    (else
      ;[1 1 1] Regeneration Health
      (if (< (`self.Health`) (`self.Health_Max`))
        (`KismetSystemLibrary.Delay` 1.0)
        (set `self.Health` (+ (`self.Health`) (`self.Health_Reg`)))))))

(fn `UserConstructionScript`)